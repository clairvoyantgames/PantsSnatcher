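; Game mode for a toilet horror game with growing pattern rounds, creating the start menu and message widgets.
; Tick builds each round's shuffled pattern from TriggerNumbers, one entry longer per level, and CyclePattern steps through it.
; A retriggerable five-second delay, restarted by early sounds, starts the round, then sound and cycle checks decide success or game over.
; Game over flashes the creep with lights off and a scream, then reloads Toilet.
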(event Custom|Cycle%20Pattern
  (Variables|Default|SetPattern%20Value (Utilities|Array|Get(acopy) (Variables|Default|GetPattern%20Order) (Variables|Default|GetCurrent%20Pattern%20Index)))
  (Math|Integer|CompareInt (Variables|Default|GetCurrent%20Pattern%20Index) (- (Utilities|Array|Length (Variables|Default|GetPattern%20Order)) 1)
    (:==
      (Variables|Default|SetCurrent%20Pattern%20Index 0))
    (:<
      (Variables|Default|SetCurrent%20Pattern%20Index (+ (Variables|Default|GetCurrent%20Pattern%20Index) 1)))))

(event EventTick
  (params (DeltaSeconds :type Float%20%28single-precision%29))
  (bind _pattern_order (Variables|Default|GetPattern%20Order))
  (if (Variables|Default|GetGame%20Over)
    (Utilities|FlowControl|DoOnce false
      (:Completed
        (Utilities|Casting|CastToBP_Player (Game|Player|GetPlayerPawn 0))
        (Rendering|SetActorHiddenInGame (Variables|Default|GetTriggered%20Creep) false)
        (Utilities|FlowControl|Delay 0.5)
        (Variables|Default|SetLights%20on false)
        (bind _asbp_player_c (Utilities|Casting|CastToBP_Player (Game|Player|GetPlayerPawn 0)))
        (Rendering|ToggleVisibility (Variables|/Game/Blueprints/BP_Player.BP_Player_C|GetPants _asbp_player_c) false)
        (Audio|Components|Audio|Play (Variables|/Game/Blueprints/BP_Player.BP_Player_C|GetScream _asbp_player_c) 0.0)
        (Utilities|FlowControl|Delay 0.5)
        (Rendering|SetActorHiddenInGame (Variables|Default|GetTriggered%20Creep) true)
        (Variables|Default|SetLights%20on true)
        (Utilities|FlowControl|Delay 2.0)
        (Game|OpenLevel(byName) "Toilet")))
    (else
      (Utilities|FlowControl|Sequence
        (:then_1
          (if (Variables|Default|GetIs%20Pattern%20Done)
            (Utilities|Array|Clear _pattern_order)
            (for _index (range 0 (- (Variables|Default|GetCurrent%20Level) 1))
              (Utilities|Array|Add _pattern_order (Utilities|Array|Get(acopy) (Variables|Default|GetTrigger%20Numbers) (Variables|Default|GetTrigger%20Number%20Index)))
              (if (== (Variables|Default|GetTrigger%20Number%20Index) (- (Utilities|Array|Length (Variables|Default|GetTrigger%20Numbers)) 1))
                (Variables|Default|SetTrigger%20Number%20Index 0)
                (else
                  (Variables|Default|SetTrigger%20Number%20Index (+ (Variables|Default|GetTrigger%20Number%20Index) 1)))))
            (Variables|Default|SetIs%20Pattern%20Done false)
            (Utilities|Array|Shuffle (Variables|Default|GetPattern%20Order))
            (Variables|Default|SetCurrent%20Level (+ (Variables|Default|GetCurrent%20Level) 1))))
        (:then_2
          (if (Variables|Default|GetGame%20Ready)
            (Utilities|FlowControl|Sequence
              (:then_0
                (goto _label_3 Reset))
              (:then_1
                (Utilities|FlowControl|DoOnce false :!label _label
                  (:Completed
                    (Utilities|FlowControl|RetriggerableDelay 5.0 :!label _label_2)
                    (Variables|Default|SetGame%20Start true)
                    (bind _asbp_message_c (Utilities|Casting|CastToBP_Message (Variables|Default|Gettext%20widget)))
                    (Default|ShowStart _asbp_message_c))))
              (:then_2
                (if (Variables|Default|GetHas%20Played%20Sound)
                  (Variables|Default|SetHas%20Played%20Sound false)
                  (if (Variables|Default|GetGame%20Start)
                    (Variables|Default|SetGame%20Over true)
                    (else
                      (goto _label_2)))
                  (elif (and (Variables|Default|GetGame%20Start) (== (Variables|Default|GetCurrent%20Level) (Variables|Default|GetPattern%20Cycles)))
                    (if (Variables|Default|GetHas%20Played%20Sound)
                      (bind _asbp_message_c_2 (Utilities|Casting|CastToBP_Message (Variables|Default|Gettext%20widget)))
                      (Default|ShowGoodJob _asbp_message_c_2)
                      (Variables|Default|SetGame%20Ready false)
                      (Variables|Default|SetGame%20Start false)
                      (Variables|Default|SetIs%20Pattern%20Done true)
                      (Variables|Default|SetPattern%20Cycles 1)
                      (Utilities|FlowControl|Delay 3.0)
                      (Variables|Default|SetGame%20Ready true)
                      (else
                        (Variables|Default|SetGame%20Over true)))))))
            (else
              (Utilities|FlowControl|Sequence
                (:then_0
                  (goto _label Reset))
                (:then_1
                  (Utilities|FlowControl|DoOnce false :!label _label_3
                    (:Completed
                      (CallFunction|CyclePattern))))))))))))

(event EventBeginPlay
  (bind _returnvalue (UserInterface|CreateWidget "/Game/Blueprints/BP_StartMenu.BP_StartMenu_C"))
  (Variables|Default|SetWidget _returnvalue)
  (UserInterface|Viewport|AddtoViewport _returnvalue)
  (bind _returnvalue_2 (UserInterface|CreateWidget "/Game/Blueprints/BP_Message.BP_Message_C"))
  (Variables|Default|Settext%20widget _returnvalue_2)
  (UserInterface|Viewport|AddtoViewport _returnvalue_2))

(fn ConstructionScript)