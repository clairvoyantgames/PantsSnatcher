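; BP_Player is the player Blueprint that plays a monster sound when the trigger matching the game mode's pattern is active.
; Each tick compares BP_GameMode's PatternValue with one to select the left, front or right trigger flag.
; All three branches share a DoOnce that fires PlaySound, which flags HasPlayedSound on the game mode, plays Monster briefly, stops it, then resets the gate.
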(event Custom|Play%20Sound
  (bind _monster (Variables|Default|GetMonster))
  (bind _asbp_gamemode_c (Utilities|Casting|CastToBP_GameMode (Game|GetGameMode)))
  (Variables|/Game/Blueprints/BP_GameMode.BP_GameMode_C|SetHas%20Played%20Sound _asbp_gamemode_c true)
  (Audio|Components|Audio|Play _monster 3.0)
  (Utilities|FlowControl|RetriggerableDelay 3.0)
  (Audio|Components|Audio|Stop _monster)
  (Utilities|FlowControl|DoOnce false) ; enters at Reset
)

(event EventTick
  (params (DeltaSeconds :type Float%20%28single-precision%29))
  (bind _asbp_gamemode_c (Utilities|Casting|CastToBP_GameMode (Game|GetGameMode)))
  (Math|Integer|CompareInt (Variables|/Game/Blueprints/BP_GameMode.BP_GameMode_C|GetPattern%20Value _asbp_gamemode_c) 1
    (:>
      (if (Variables|Default|GetRight%20Triggered)
        (Utilities|FlowControl|DoOnce false :!label _label
          (:Completed
            (CallFunction|PlaySound)))))
    (:==
      (if (Variables|Default|GetFront%20Triggered)
        (goto _label)))
    (:<
      (if (Variables|Default|GetLeft%20Triggered)
        (goto _label)))))

(fn ConstructionScript)