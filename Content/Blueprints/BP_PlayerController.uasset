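; Player controller that moves the BP_Player pawn, either by foot-direction input or by following the mouse, and maps axis input to pitch and yaw.
; Four Feet actions set a foot index, which Tick maps to a preset location and snaps the pawn there while StartPressed is true.
; Otherwise, Tick traces under the cursor and interpolates the pawn toward the hit's XY with sweep.
; Movement stops when BP_GameMode has both GameOver and GameReady set.
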(event EventTick
  (params (DeltaSeconds :type Float%20%28single-precision%29))
  (bind (_worldlocation _worlddirection) (Game|Player|ConvertMouseLocationToWorldSpace))
  (bind _returnvalue (Pawn|GetControlledPawn))
  (bind _current_foot_location (Variables|Default|GetCurrent%20Foot%20Location))
  (bind _asbp_gamemode_c (Utilities|Casting|CastToBP_GameMode (Game|GetGameMode)))
  (if (not (and (Variables|/Game/Blueprints/BP_GameMode.BP_GameMode_C|GetGame%20Over _asbp_gamemode_c) (Variables|/Game/Blueprints/BP_GameMode.BP_GameMode_C|GetGame%20Ready _asbp_gamemode_c)))
    (if (Variables|Default|GetStart%20Pressed)
      (Math|Integer|CompareInt _current_foot_location 1
        (:>
          (Variables|Default|SetCurrent%20Location (Variables|Default|GetRight%20Location)))
        (:==
          (Variables|Default|SetCurrent%20Location (Variables|Default|GetFront%20Location)))
        (:<
          (if (== _current_foot_location 0)
            (Variables|Default|SetCurrent%20Location (Variables|Default|GetLeft%20Location))
            (else
              (Variables|Default|SetCurrent%20Location (Variables|Default|GetDefault%20Location))))))
      (Utilities|Casting|CastToBP_Player _returnvalue)
      (Transformation|SetActorLocation _returnvalue (Variables|Default|GetCurrent%20Location) false)
      (else
        (bind _asbp_player_c (Utilities|Casting|CastToBP_Player (Pawn|GetControlledPawn)))
        (bind _outhit (Collision|LineTraceForObjects _worldlocation (+ _worldlocation (* _worlddirection 4e+04)) (Variables|Default|GetObject%20Types) false 0 "None"))
        (Transformation|SetActorLocation _asbp_player_c (Math|Interpolation|VInterpTo (Transformation|GetActorLocation _asbp_player_c) (Math|Vector|MakeVector (.X (Math|Vector|BreakVector (.Location (Collision|BreakHitResult _outhit)))) (.Y (Math|Vector|BreakVector (.Location (Collision|BreakHitResult _outhit)))) (.Z (Math|Vector|BreakVector (Transformation|GetActorLocation _asbp_player_c)))) DeltaSeconds (Variables|Default|GetMove%20Speed)) true)))))

(event Input|ActionEvents|InputActionFeetUp
  (:Pressed
    (Variables|Default|SetCurrent%20Foot%20Location 2)))

(event Input|ActionEvents|InputActionFeetBack
  (:Pressed
    (Variables|Default|SetCurrent%20Foot%20Location -1)))

(event Input|ActionEvents|InputActionFeetLeft
  (:Pressed
    (Variables|Default|SetCurrent%20Foot%20Location 0)))

(event Input|ActionEvents|InputActionFeetRight
  (:Pressed
    (Variables|Default|SetCurrent%20Foot%20Location 1)))

(event Input|AxisEvents|InputAxisMoveUp
  (params (AxisValue :type Float%20%28single-precision%29))
  (Class|PlayerController|AddPitchInput AxisValue))

(event Input|AxisEvents|InputAxisMoveLeft
  (params (AxisValue :type Float%20%28single-precision%29))
  (Class|PlayerController|AddYawInput AxisValue))

(fn ConstructionScript)